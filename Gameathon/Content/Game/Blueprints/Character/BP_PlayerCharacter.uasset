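; First-person player character with two-handed pickup and use of interactables, notably a Dalla pot (left hand) and cups (right hand).
; A looping timer sphere-traces from the camera to toggle the interaction prompt widget.
; Pickup input traces to grab or drop per hand, or refills the held cup from the Dalla on left input; interact uses a held item.
; Helpers expose smoothed movement input and hand wall traces, likely for arm animation.
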(event Input|EnhancedActionEvents|EnhancedInputActionIA_Move
  (params (ActionValue :type Vector%202D%20Structure) (ElapsedSeconds :type Float%20%28double-precision%29) (TriggeredSeconds :type Float%20%28double-precision%29) (InputAction :type Input%20Action%20Object%20Reference :default "/Game/Game/Blueprints/Input/IA_Move.IA_Move"))
  ;[1 1 1] Mouse
  (:Triggered
    (Pawn|Input|AddMovementInput (Transformation|GetActorRightVector) (.x ActionValue) false)
    (Pawn|Input|AddMovementInput (Transformation|GetActorForwardVector) (.y ActionValue) false)))

(event Input|EnhancedActionEvents|EnhancedInputActionIA_Look
  (params (ActionValue :type Vector%202D%20Structure) (ElapsedSeconds :type Float%20%28double-precision%29) (TriggeredSeconds :type Float%20%28double-precision%29) (InputAction :type Input%20Action%20Object%20Reference :default "/Game/Game/Blueprints/Input/IA_Look.IA_Look"))
  ;[1 1 1] Look
  (:Triggered
    (Pawn|Input|AddControllerYawInput (.x ActionValue))
    (Pawn|Input|AddControllerPitchInput (.y ActionValue))))

(event Input|EnhancedActionEvents|EnhancedInputActionIA_PickupItem
  (params (ActionValue :type Float%20%28double-precision%29) (ElapsedSeconds :type Float%20%28double-precision%29) (TriggeredSeconds :type Float%20%28double-precision%29) (InputAction :type Input%20Action%20Object%20Reference :default "/Game/Game/Blueprints/Input/IA_PickupItem.IA_PickupItem"))
  ;[1 1 1] Interact
  (:Started
    (CallFunction|InteractionTrace (select (> ActionValue 0.0) "NewEnumerator0" "NewEnumerator1"))))

(event Input|EnhancedActionEvents|EnhancedInputActionIA_InteractItem
  (params (ActionValue :type Boolean) (ElapsedSeconds :type Float%20%28double-precision%29) (TriggeredSeconds :type Float%20%28double-precision%29) (InputAction :type Input%20Action%20Object%20Reference :default "/Game/Game/Blueprints/Input/IA_InteractItem.IA_InteractItem"))
  ;[1 1 1] Interact
  (:Started
    (bind _interactedactorleft (Variables|Default|GetInteractedActorLeft)
      (:then
        (Class|BPIInteractable|Interact(Message) _interactedactorleft))
      (:else
        (bind _interactedactorright (Variables|Default|GetInteractedActorRight)
          (:then
            (Class|BPIInteractable|Interact(Message) _interactedactorright))
          (:else))))))

(event EventBeginPlay
  (bind _returnvalue (Game|GetPlayerController 0))
  (bind _returnvalue_2 (PlayerController|LocalPlayerSubsystems|GetEnhancedInputLocalPlayerSubsystem _returnvalue))
  ;[1 1 1] Initialize
  (Utilities|IsValid _returnvalue_2
    (:Is%20Valid
      (Input|AddMappingContext _returnvalue_2 "/Game/Game/Blueprints/Input/IM_Gameplay.IM_Gameplay" 0 "(bIgnoreAllPressedKeysUntilRelease=True,bForceImmediately=False)")
      (Utilities|Time|SetTimerbyFunctionName 0 "CheckForInteractables" 0.01 true))))

(fn ConstructionScript)

(fn InteractionTrace
  (params (Hand :type E_Hand%20Enum :default "NewEnumerator0"))
  (bind _camera (Variables|Default|GetCamera))
  (bind _returnvalue (Transformation|GetWorldLocation _camera))
  (switch Utilities|FlowControl|Switch|SwitchonE_Hand Hand
    (:NewEnumerator0
      (bind _interactedactorright (Variables|Default|GetInteractedActorRight)
        (:then
          (bind _asbp_interactable_dalla (Utilities|Casting|CastToBP_Interactable_Dalla (Variables|Default|GetInteractedActorLeft))
            (:then
              (bind _asbp_interactable_cup (Utilities|Casting|CastToBP_Interactable_Cup _interactedactorright)
                (:then
                  (Default|RefillFinjal _asbp_interactable_dalla _asbp_interactable_cup))
                (:CastFailed
                  (bind (_outhit _returnvalue_2) (Collision|SphereTraceByChannel _returnvalue (+ _returnvalue (* (Math|Vector|GetForwardVector _camera) (Variables|Default|GetInteractDistance))) 5.0 "TraceTypeQuery1" false 0 "None" :!label _label))
                  (if _returnvalue_2
                    (if (Utilities|DoesObjectImplementInterface (.HitActor (Collision|BreakHitResult _outhit)) "/Game/Game/Blueprints/Interfaces/BPI_Interactable.BPI_Interactable_C")
                      (bind _canpickup (Class|BPIInteractable|IsPickupable(Message) (.HitActor (Collision|BreakHitResult _outhit))))
                      (if _canpickup
                        (bind _asbp_interactable_cup_2 (Utilities|Casting|CastToBP_Interactable_Cup (.HitActor (Collision|BreakHitResult _outhit)))
                          (:then
                            (CallFunction|Pickup _asbp_interactable_cup_2 "NewEnumerator1"))
                          (:CastFailed
                            (bind _asbp_interactable_dalla_2 (Utilities|Casting|CastToBP_Interactable_Dalla (.HitActor (Collision|BreakHitResult _outhit))))
                            (CallFunction|Pickup _asbp_interactable_dalla_2 "NewEnumerator0")))
                        (else
                          (Class|BPIInteractable|Pickup(Message) (.HitActor (Collision|BreakHitResult _outhit)) Hand)))
                      (else
                        (CallFunction|ShouldDropItem Hand :!label _label_2)))
                    (else
                      (goto _label_2))))))
            (:CastFailed
              (goto _label))))
        (:else
          (goto _label))))
    (:NewEnumerator1
      (goto _label))))

(fn CheckforInteractables
  (bind _camera (Variables|Default|GetCamera))
  (bind _returnvalue (Transformation|GetWorldLocation _camera))
  (bind (_outhit _returnvalue_2) (Collision|SphereTraceByChannel _returnvalue (+ _returnvalue (* (Math|Vector|GetForwardVector _camera) (Variables|Default|GetInteractDistance))) 5.0 "TraceTypeQuery1" false 0 "None"))
  (if _returnvalue_2
    (if (Utilities|DoesObjectImplementInterface (.HitActor (Collision|BreakHitResult _outhit)) "/Game/Game/Blueprints/Interfaces/BPI_Interactable.BPI_Interactable_C")
      (Class|BPIInteractable|OnLook(Message) (.HitActor (Collision|BreakHitResult _outhit)))
      (Variables|Default|GetWInteraction
        (:then
          (if (not (UserInterface|Viewport|IsinViewport (Variables|Default|GetWInteraction)))
            (UserInterface|Viewport|AddtoViewport (stale _output_get) 0 :!label _label)))
        (:else
          (bind _isleft (Class|BPIInteractable|IsLeftPickup(Message) (.HitActor (Collision|BreakHitResult _outhit))))
          (bind _returnvalue_3 (UserInterface|CreateWidget "/Game/Game/UI/Gameplay/W_Interaction.W_Interaction_C" 0 _isleft))
          (bind _output_get (Variables|Default|SetWInteraction _returnvalue_3))
          (goto _label)))
      (else
        (Variables|Default|GetWInteraction :!label _label_2
          (:then
            (Widget|RemovefromParent (Variables|Default|GetWInteraction))
            (Variables|Default|SetWInteraction 0))
          (:else))))
    (else
      (goto _label_2))))

(fn ShouldDropItem
  (params (Hand :type E_Hand%20Enum :default "NewEnumerator0"))
  (switch Utilities|FlowControl|Switch|SwitchonE_Hand Hand
    (:NewEnumerator0
      (bind _interactedactorleft (Variables|Default|GetInteractedActorLeft)
        (:then
          (Class|BPIInteractable|Release(Message) _interactedactorleft)
          (Variables|Default|SetInteractedActorLeft 0))
        (:else)))
    (:NewEnumerator1
      (bind _interactedactorright (Variables|Default|GetInteractedActorRight)
        (:then
          (Class|BPIInteractable|Release(Message) _interactedactorright)
          (Variables|Default|SetInteractedActorRight 0))
        (:else)))))

(fn Pickup
  (params (Item :type Actor%20Object%20Reference) (Index :type E_Hand%20Enum :default "NewEnumerator0"))
  (CallFunction|ShouldDropItem Index)
  (switch Utilities|FlowControl|Switch|SwitchonE_Hand Index
    (:NewEnumerator0
      (Variables|Default|SetInteractedActorLeft Item))
    (:NewEnumerator1
      (Variables|Default|SetInteractedActorRight Item)))
  (Class|BPIInteractable|Pickup(Message) Item Index))

(fn GetHeldItem
  (params (Hand :type E_Hand%20Enum :default "NewEnumerator0"))
  (return (Utilities|Select :Index Hand :NewEnumerator0 (Variables|Default|GetInteractedActorLeft) :NewEnumerator1 (Variables|Default|GetInteractedActorRight))))

(fn GetMovementInput
  (bind _returnvalue (Input|EnhancedActionValues|GetIA_Move))
  (Variables|Default|SetTurnDelta (Math|Interpolation|FInterpTo (Variables|Default|GetTurnDelta) (.x (Input|EnhancedActionValues|GetIA_Look)) (Utilities|Time|GetWorldDeltaSeconds) 1e+01))
  (return (Math|Vector2D|MakeVector2D (.y _returnvalue) (.x _returnvalue)) (* (Variables|Default|GetTurnDelta) 15.0)))

(fn GetPlayerMesh
  (return (Variables|Default|GetSK_Arms)))

(fn HandWallTrace
  (params (StartingSocket :type Name :default "None") (InSocketName :type Name :default "None") (TraceLength :type Float%20%28double-precision%29))
  (bind _sk_arms (Variables|Default|GetSK_Arms))
  (bind _camera (Variables|Default|GetCamera))
  (bind _returnvalue (Math|Vector|GetForwardVector _camera))
  (bind _returnvalue_2 (Transformation|GetSocketTransform _sk_arms InSocketName "RTS_World"))
  (bind (_outhit _returnvalue_3) (Collision|SphereTraceByChannel (.location _returnvalue_2) (+ (.location _returnvalue_2) (* _returnvalue TraceLength)) 5.0 "TraceTypeQuery2" true 0 "None"))
  (return _returnvalue_3 (+ (.Location (Collision|BreakHitResult _outhit)) (* _returnvalue (Math|Float|SelectFloat 15.0 -15.0 (< TraceLength 0.0))))))
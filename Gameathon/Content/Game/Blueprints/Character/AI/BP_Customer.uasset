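; AI coffee shop customer that draws a name from the GameState pool and orders one or two coffees.
; When seated, it anticipates coffee and turns its head toward the player; a timer billboards its alert widget.
; Pickup attaches the player's cup to its hand, sipping full cups and rejecting others, or returns finished cups.
; Drinks increment CoffeesServed; once satisfied, it returns its name, walks to a TargetPoint and is destroyed.
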(event Custom|ExitRoom
  ;[1 1 1] Force customer to leave room
  (bind _asbp_game_state (Utilities|Casting|CastToBP_GameState (Game|GetGameState)))
  (Utilities|Array|Add (Variables|/Game/Game/Blueprints/Core/BP_GameState.BP_GameState_C|GetCustomerNames _asbp_game_state) (.name (Variables|Default|GetCustomerData)))
  (CallFunction|UpdateSeated false)
  (Utilities|FlowControl|Delay 3.0)
  (bind _returnvalue (Actor|GetActorOfClass "/Script/Engine.TargetPoint"))
  (AI|AIMoveTo (AI|GetAIController self) "0, 0, 0" _returnvalue -1.0 "Default" "Default" true true
    (:OnMoveFinished
      (Actor|DestroyActor))))

(event Custom|FinishedDrink
  ;[1 1 1] Give customer coffeee
  ;;[1 1 1] Call when drink is finished
  (Utilities|FlowControl|DoOnce false) ; enters at Reset
)

(event Custom|SipDrink
  (bind _customerdata (Variables|Default|GetCustomerData))
  (bind _customerdata_2 (Variables|Default|GetCustomerData))
  (bind _returnvalue (<= (.coffees _customerdata_2) 0))
  (Animation|Montage|PlayMontage (Variables|Character|GetMesh) "/Game/Game/Art/Character/Montages/M_DrinkCoffee.M_DrinkCoffee"
    (:OnBlendOut
      (Default|CallOnFinjalStateChange (Variables|Default|GetCupRef) "NewEnumerator2")
      (Default|CallOnItemStateUpdated (Variables|Default|GetCupRef) false)
      (|SetBy-RefVar (.coffees _customerdata) (Math|Integer|Clamp(Integer) (- (.coffees _customerdata) 1) 0 100))
      (Default|CallOnFinishedDrink)
      (Variables|Default|SetDrinkFinished true)
      (Rendering|SetVisibility (Variables|Default|GetAlertWidget) (not _returnvalue) false)
      (if (not _returnvalue)
        (CallFunction|WantingCoffee)))))

(event Custom|WantingCoffee
  (bind _returnvalue (Game|GetPlayerCharacter 0))
  (bind _mesh (Variables|Character|GetMesh))
  (bind _returnvalue_2 (Transformation|GetSocketLocation _mesh "Head"))
  (bind _returnvalue_3 (Transformation|GetActorLocation _returnvalue))
  (bind _returnvalue_4 (Math|Rotator|FindLookatRotation _returnvalue_2 _returnvalue_3))
  (Animation|PlayAnimMontage "/Game/Game/Art/Character/Montages/M_AnticipateCoffee.M_AnticipateCoffee" 1.0 "None")
  (Utilities|FlowControl|Gate true) ; enters at Open
)

(event Custom|OnFinishedDrink_Event
  (bind _asbp_game_state (Utilities|Casting|CastToBP_GameState (Game|GetGameState)))
  (Variables|/Game/Game/Blueprints/Core/BP_GameState.BP_GameState_C|SetCoffeesServed _asbp_game_state (+ (Variables|/Game/Game/Blueprints/Core/BP_GameState.BP_GameState_C|GetCoffeesServed _asbp_game_state) 1)))

(event Custom|HandBackGlass
  (Default|CallOnItemStateUpdated (Variables|Default|GetCupRef) false)
  (Variables|Default|SetDrinkFinished true)
  (Rendering|SetVisibility (Variables|Default|GetAlertWidget) true false)
  (CallFunction|WantingCoffee))

(event EventBeginPlay
  (CallFunction|GenerateCustomerData)
  (Utilities|Time|SetTimerbyFunctionName 0 "SwivelAlertWidget" 0.01 true)
  (EventDispatchers|BindEventtoOnFinishedDrink (delegate Custom|OnFinishedDrink_Event)))

(event EventPickup
  (params (Hand :type E_Hand%20Enum :default "NewEnumerator0"))
  ;[1 1 1] Give customer coffeee
  (Variables|Default|GetCupRef
    (:then
      (if (Variables|Default|GetDrinkFinished)
        (bind _asbp_player_character (Utilities|Casting|CastToBP_PlayerCharacter (Game|Player|GetPlayerPawn 0)))
        (Default|Pickup _asbp_player_character (Variables|Default|GetCupRef) "NewEnumerator1")
        (Variables|Default|SetCupRef 0)
        (if (<= (.coffees (Variables|Default|GetCustomerData)) 0)
          (CallFunction|ExitRoom)
          (else
            (CallFunction|FinishedDrink)))
        (Variables|Default|SetDrinkFinished false)))
    (:else
      (if (Variables|Default|GetbIsSeated)
        (bind _item (Class|BPICharacter|GetHeldItem(Message) (Game|Player|GetPlayerPawn 0) Hand))
        (Utilities|IsValid _item
          (:Is%20Valid
            (bind _asbp_interactable_cup (Utilities|Casting|CastToBP_Interactable_Cup _item))
            (Utilities|FlowControl|DoOnce false
              (:Completed
                (Transformation|DetachFromActor _asbp_interactable_cup "KeepWorld" "KeepWorld" "KeepWorld")
                (bind _asbp_player_character_2 (Utilities|Casting|CastToBP_PlayerCharacter (Game|Player|GetPlayerPawn 0)))
                (switch Utilities|FlowControl|Switch|SwitchonE_Hand Hand
                  (:NewEnumerator0
                    (Variables|/Game/Game/Blueprints/Character/BP_PlayerCharacter.BP_PlayerCharacter_C|SetInteractedActorLeft _asbp_player_character_2 0))
                  (:NewEnumerator1
                    (Variables|/Game/Game/Blueprints/Character/BP_PlayerCharacter.BP_PlayerCharacter_C|SetInteractedActorRight _asbp_player_character_2 0)))
                (Transformation|AttachComponentToComponent _asbp_interactable_cup (Variables|Character|GetMesh) "s_item_cup" "SnapToTarget" "SnapToTarget" "SnapToTarget" false)
                (bind _output_get (Variables|Default|SetCupRef _asbp_interactable_cup))
                (Collision|SetCollisionProfileName (Variables|/Game/Game/Blueprints/Gameplay/Items/BP_Interactable_Cup.BP_Interactable_Cup_C|GetFingan_Coffee_Cup _output_get) "PhysicsActor" true :!class /Script/Engine.PrimitiveComponent)
                (Animation|StopAnimMontage "/Game/Game/Art/Character/Montages/M_AnticipateCoffee.M_AnticipateCoffee")
                (Variables|Default|SetDrinkFinished false)
                (Rendering|SetVisibility (Variables|Default|GetAlertWidget) false false)
                (switch Utilities|FlowControl|Switch|SwitchonE_FinjalState (Variables|/Game/Game/Blueprints/Gameplay/Items/BP_Interactable_Cup.BP_Interactable_Cup_C|GetFinjalState (Variables|Default|GetCupRef))
                  (:NewEnumerator3
                    (CallFunction|HandBackGlass :!label _label)
                    (bind _asbp_game_state (Utilities|Casting|CastToBP_GameState (Game|GetGameState)))
                    (Default|CallOnSendMessage _asbp_game_state "You're serving coffee not empty cups!" 5.0))
                  (:NewEnumerator0
                    (goto _label))
                  (:NewEnumerator1
                    (CallFunction|SipDrink))
                  (:NewEnumerator2
                    (goto _label)))))))))))

(event EventUpdateSeated
  (params (Seated :type Boolean))
  (bind _output_get (Variables|Default|SetbIsSeated Seated))
  (if _output_get
    (CallFunction|WantingCoffee)
    (else
      (Animation|StopAnimMontage "/Game/Game/Art/Character/Montages/M_AnticipateCoffee.M_AnticipateCoffee"))))

(event EventTick
  (params (DeltaSeconds :type Float%20%28single-precision%29))
  (bind _returnvalue (Game|GetPlayerCharacter 0))
  (bind _mesh (Variables|Character|GetMesh))
  (bind _returnvalue_2 (Transformation|GetSocketLocation _mesh "Head"))
  (bind _returnvalue_3 (Transformation|GetActorLocation _returnvalue))
  (bind _returnvalue_4 (Math|Rotator|FindLookatRotation _returnvalue_2 _returnvalue_3))
  (Utilities|FlowControl|Gate true
    (:Exit
      (Variables|Default|SetHeadRotation (Math|Rotator|MakeRotator 9e+01 0.0 (Math|Float|Clamp(Float) (.yaw (Math|Rotator|CombineRotators (Math|Rotator|MakeRotator (.roll _returnvalue_4) (.pitch _returnvalue_4) (+ (* (.yaw _returnvalue_4) -1.0) 9e+01)) (Transformation|GetWorldRotation _mesh))) -9e+01 9e+01))))))

(fn ConstructionScript)

(fn SwivelAlertWidget
  (Transformation|SetWorldRotation (Variables|Default|GetAlertWidget) (Math|Rotator|FindLookatRotation (Transformation|GetActorLocation) (Camera|GetCameraLocation (Game|GetPlayerCameraManager 0))) false false))

(fn GenerateCustomerData
  (bind _asbp_game_state (Utilities|Casting|CastToBP_GameState (Game|GetGameState)))
  (bind _output_get (LocalVariables|SetChosenName (.OutItem (Utilities|Array|Random (Variables|/Game/Game/Blueprints/Core/BP_GameState.BP_GameState_C|GetCustomerNames _asbp_game_state)))))
  (Variables|Default|SetCustomerData (Utilities|Struct|MakeS_CustomerData _output_get "NewEnumerator0" (Math|Random|RandomIntegerinRange 1 2)))
  (Utilities|Array|RemoveItem (Variables|/Game/Game/Blueprints/Core/BP_GameState.BP_GameState_C|GetCustomerNames _asbp_game_state) (LocalVariables|GetChosenName)))

(fn GetHandIK
  (return "0, 0, 0" "0, 0, 0"))

(fn GetItemSocket
  (return "None"))

(fn IsLeftPickup
  (return false))

(fn IsPickupable
  (return false))
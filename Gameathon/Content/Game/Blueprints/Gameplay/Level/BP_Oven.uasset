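; BP_Oven is a non-pickupable level interactable that refills the Dallah the player is holding.
; Its Pickup event checks the player character's left interacted actor and calls RefillDallah when it is a BP_Interactable_Dalla.
; Any other valid left-hand actor triggers a timed hint message through BP_GameState, while an empty left hand does nothing.
; Socket and hand IK queries return empty defaults.
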(event EventBeginPlay)

(event Collision|EventActorBeginOverlap
  (params (OtherActor :type Actor%20Object%20Reference)))

(event EventTick
  (params (DeltaSeconds :type Float%20%28single-precision%29)))

(event EventPickup
  (params (Hand :type E_Hand%20Enum :default "NewEnumerator0"))
  (bind _asbp_player_character (Utilities|Casting|CastToBP_PlayerCharacter (Game|Player|GetPlayerPawn 0)))
  (bind _interactedactorleft (Variables|/Game/Game/Blueprints/Character/BP_PlayerCharacter.BP_PlayerCharacter_C|GetInteractedActorLeft _asbp_player_character)
    (:then
      (bind _asbp_interactable_dalla (Utilities|Casting|CastToBP_Interactable_Dalla _interactedactorleft)
        (:then
          (Default|RefillDallah _asbp_interactable_dalla))
        (:CastFailed
          (bind _asbp_game_state (Utilities|Casting|CastToBP_GameState (Game|GetGameState)))
          (Default|CallOnSendMessage _asbp_game_state "The Finjal uses the Dallah silly..." 5.0))))
    (:else)))

(fn ConstructionScript)

(fn GetHandIK
  (return "0, 0, 0" "0, 0, 0"))

(fn GetItemSocket
  (return "None"))

(fn IsLeftPickup
  (return false))

(fn IsPickupable
  (return false))
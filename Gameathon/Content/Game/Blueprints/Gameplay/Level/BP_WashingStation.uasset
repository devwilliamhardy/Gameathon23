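; BP_WashingStation is a fixed interactable station where the player cleans cups.
; On Pickup it queries player pawn 0 for the item in the given hand and calls AttemptCleanCup if that item is a BP_Interactable_Cup.
; Otherwise it sends a timed "doesn't need to be washed" message through BP_GameState.
; Its pickup query functions return empty defaults, marking it as not pickupable.
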(event EventBeginPlay)

(event Collision|EventActorBeginOverlap
  (params (OtherActor :type Actor%20Object%20Reference)))

(event EventTick
  (params (DeltaSeconds :type Float%20%28single-precision%29)))

(event EventPickup
  (params (Hand :type E_Hand%20Enum :default "NewEnumerator0"))
  (bind _item (Class|BPICharacter|GetHeldItem(Message) (Game|Player|GetPlayerPawn 0) Hand))
  (bind _asbp_interactable_cup (Utilities|Casting|CastToBP_Interactable_Cup _item)
    (:then
      (Default|AttemptCleanCup _asbp_interactable_cup))
    (:CastFailed
      (bind _asbp_game_state (Utilities|Casting|CastToBP_GameState (Game|GetGameState)))
      (Default|CallOnSendMessage _asbp_game_state "This item doesn't need to be washed." 5.0))))

(fn ConstructionScript)

(fn GetHandIK
  (return "0, 0, 0" "0, 0, 0"))

(fn GetItemSocket
  (return "None"))

(fn IsLeftPickup
  (return false))

(fn IsPickupable
  (return false))
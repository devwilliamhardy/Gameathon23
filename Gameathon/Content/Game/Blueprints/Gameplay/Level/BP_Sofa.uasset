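; BP_Sofa is a level actor that seats a customer pawn.
; HandleSittingDown plays a timeline that blends the pawn's location, rotation and scale toward the CustomerTransform component, lerping from its current transform each update rather than a cached start.
; When the timeline finishes, it notifies BP_GameState with the pawn and sofa, then turns on the pawn's seated message.
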(event Custom|HandleSittingDown
  (params (Pawn :type Pawn%20Object%20Reference))
  (bind _alpha (Timeline|TL_MoveCustomer PlayFromStart)
    (:Update
      (Transformation|SetActorTransform Pawn (Math|Transform|MakeTransform (.location (Math|Transform|Lerp(Transform) (Transformation|GetActorTransform Pawn) (Transformation|GetWorldTransform (Variables|Default|GetCustomerTransform)) _alpha)) (.rotation (Math|Transform|Lerp(Transform) (Transformation|GetActorTransform Pawn) (Transformation|GetWorldTransform (Variables|Default|GetCustomerTransform)) _alpha)) (.scale (Math|Transform|Lerp(Transform) (Transformation|GetActorTransform Pawn) (Transformation|GetWorldTransform (Variables|Default|GetCustomerTransform)) _alpha)))))
    (:Finished
      (bind _asbp_game_state (Utilities|Casting|CastToBP_GameState (Game|GetGameState)))
      (Default|HandleCustomerSittingDown _asbp_game_state Pawn self)
      (Class|BPIInteractable|UpdateSeated(Message) Pawn true))))

(event EventBeginPlay)

(event Collision|EventActorBeginOverlap
  (params (OtherActor :type Actor%20Object%20Reference)))

(event EventTick
  (params (DeltaSeconds :type Float%20%28single-precision%29)))

(fn ConstructionScript)
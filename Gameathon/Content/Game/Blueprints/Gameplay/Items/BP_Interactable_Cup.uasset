(event Custom|AttemptCleanCup
  ;[1 1 1] Clean
  (Default|CallOnFinjalStateChange "NewEnumerator3")
  (Audio|PlaySoundatLocation "/Game/Game/Audio/PutCupToClean_Cue.PutCupToClean_Cue" (Transformation|GetActorLocation) "0, 0, 0" 1.0 (Math|Random|RandomFloatinRange 0.8 1.1) 0.0 0 0 0 0)
  (Variables|Default|SetInitiallyDirty false))

(event Custom|HandleFinjalFinjalState
  (params (State :type E_FinjalState%20Enum :default "NewEnumerator3"))
  (bind _output_get (Variables|Default|SetFinjalState State))
  (Components|StaticMesh|SetStaticMesh (Variables|Default|GetFingan_Coffee_Cup) (Utilities|Select :Index _output_get :NewEnumerator3 "/Game/Game/Art/Gameplay/New_Fingan.New_Fingan" :NewEnumerator0 "/Game/Game/Art/Gameplay/New_Fingan.New_Fingan" :NewEnumerator1 "/Game/Game/Art/Gameplay/Filled_Fingan.Filled_Fingan" :NewEnumerator2 "/Game/Game/Art/Gameplay/Used_Fingan.Used_Fingan")))

(event Custom|FillFinjal
  (bind _finjalstate (Variables|Default|GetFinjalState))
  ;[1 1 1] Fill
  (if (or (Utilities|Enum|Equal(Enum) _finjalstate "NewEnumerator2") (Utilities|Enum|Equal(Enum) _finjalstate "NewEnumerator3"))
    (Default|CallOnFinjalStateChange "NewEnumerator1")
    (Audio|PlaySoundatLocation "/Game/Game/Audio/Pouring_Cue.Pouring_Cue" (Transformation|GetActorLocation) "0, 0, 0" 1.0 (Math|Random|RandomFloatinRange 0.8 1.1) 0.0 0 0 0 0)
    (else
      (bind _asbp_game_state (Utilities|Casting|CastToBP_GameState (Game|GetGameState)))
      (Default|CallOnSendMessage _asbp_game_state "CLEAN YOUR FINJAL!" 5.0))))

(event EventBeginPlay
  (|CallParentFunction)
  (EventDispatchers|BindEventtoOnFinjalStateChange (EventDispatchers|CreateEvent :!event Custom|HandleFinjalFinjalState))
  (bind _asw_finjal_state (Utilities|Casting|CastToW_Finjal_State (UserInterface|GetWidget (Variables|Default|GetW_Capacity))))
  (Default|BindFinjal _asw_finjal_state self)
  (Default|CallOnFinjalStateChange "NewEnumerator2")
  (Variables|Default|SetInitiallyDirty true))

(event EventPickedUp
  (Rendering|SetVisibility (Variables|Default|GetW_Capacity) (Variables|Default|GetbIsHeld) false)
  (if (Variables|Default|GetbIsHeld)
    (Audio|PlaySoundatLocation (.OutItem (Utilities|Array|Random (Utilities|Array|MakeArray "/Game/Game/Audio/CollectCup_Cue.CollectCup_Cue" "/Game/Game/Audio/PullOutCup_Cue.PullOutCup_Cue"))) (Transformation|GetActorLocation) "0, 0, 0" 1.0 (Math|Random|RandomFloatinRange 0.8 1.1) 0.0 0 0 0 0)))

(fn ConstructionScript
  (|CallParentFunction))

(fn IsLeftPickup
  (return false))
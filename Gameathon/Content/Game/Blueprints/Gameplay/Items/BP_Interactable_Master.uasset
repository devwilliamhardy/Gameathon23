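; Base interactable item actor that the player picks up, holds and drops, with overridable pickup, look and interact hooks.
; Pickup disables mesh collision, timeline-lerps the actor to a left or right hand socket on the player mesh, then attaches it.
; Release detaches it, places it upright using camera-forward and downward capsule traces, then restores collision.
; The SetSimulatePhysics call and look-at rotation logic are disconnected and never run.
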(event Custom|HandleItemStateUpdated
  (params (PickedUp :type Boolean))
  ;[1 1 1] Handle item being picked up
  (Variables|Default|SetbIsHeld PickedUp)
  (CallFunction|PickedUp)
  (CallFunction|OnPickup))

(event Custom|DropItem
  ;[1 1 1] Hold Item
  (bind _alpha (Timeline|TL_MoveTo Stop)
    (:Update
      (Transformation|SetActorTransform (Math|Transform|Lerp(Transform) (Transformation|GetActorTransform) (Transformation|GetSocketTransform (stale EventPickup _mesh) (Utilities|String|StringToName (Utilities|String|Append (Utilities|String|ToString(Name) (Variables|Default|GetHeldSocket)) (Utilities|Select :Index (stale EventPickup Hand) :NewEnumerator0 "_l" :NewEnumerator1 "_r"))) "RTS_World") _alpha) false true))
    (:Finished
      (Transformation|AttachComponentToComponent (stale EventPickup _mesh) (Utilities|String|StringToName (Utilities|String|Append (Utilities|String|ToString(Name) (Variables|Default|GetHeldSocket)) (Utilities|Select :Index (stale EventPickup Hand) :NewEnumerator0 "_l" :NewEnumerator1 "_r"))) "SnapToTarget" "SnapToTarget" "KeepRelative" false)
      (Default|CallOnItemStateUpdated true))))

(event Custom|PickedUp
  ;[1 1 1] On look
  (bind _alpha (Timeline|TL_Return Stop)
    (:Update
      (Transformation|SetActorRelativeRotation (Math|Rotator|Lerp(Rotator) (Variables|/Script/Engine.SceneComponent|GetRelativeRotation (Variables|Default|GetDefaultSceneRoot)) (Variables|Default|GetInitialRotation) _alpha true)))))

(event Custom|TogglePhysicsExternal
  (params (bSimulate :type Boolean))
  (Utilities|TogglePhysics bSimulate))

(event Custom|OnPickup)

(event Custom|HandleInteract
  ;[1 1 1] Overridable interact
)

(event EventBeginPlay
  (EventDispatchers|BindEventtoOnItemStateUpdated (EventDispatchers|CreateEvent :!event Custom|HandleItemStateUpdated))
  (Variables|Default|SetInitialRotation (Transformation|GetActorRotation)))

(event EventOnLook
  ;[1 1 1] On look
)

(event EventPickup
  (params (Hand :type E_Hand%20Enum :default "NewEnumerator0"))
  (bind _returnvalue (Game|Player|GetPlayerPawn 0))
  (bind _returnvalue_2 (Utilities|Select :Index Hand :NewEnumerator0 "_l" :NewEnumerator1 "_r"))
  (bind _heldsocket (Variables|Default|GetHeldSocket))
  (bind _returnvalue_3 (Utilities|String|ToString(Name) _heldsocket))
  (bind _returnvalue_4 (Utilities|String|Append _returnvalue_3 _returnvalue_2))
  (bind _returnvalue_5 (Utilities|String|StringToName _returnvalue_4))
  ;[1 1 1] Hold Item
  (Utilities|IsValid _returnvalue
    (:Is%20Valid
      (Utilities|TogglePhysics false
        (:Completed
          (bind _mesh (Class|BPICharacter|GetPlayerMesh(Message) _returnvalue))
          (bind _alpha (Timeline|TL_MoveTo PlayFromStart)
            (:Update
              (Transformation|SetActorTransform (Math|Transform|Lerp(Transform) (Transformation|GetActorTransform) (Transformation|GetSocketTransform _mesh _returnvalue_5 "RTS_World") _alpha) false true))
            (:Finished
              (Transformation|AttachComponentToComponent _mesh _returnvalue_5 "SnapToTarget" "SnapToTarget" "KeepRelative" false)
              (Default|CallOnItemStateUpdated true))))))))

(event EventInteract
  ;[1 1 1] Overridable interact
  (CallFunction|HandleInteract))

(event EventRelease
  ;[1 1 1] Release Item
  (CallFunction|DropItem)
  (Default|CallOnItemStateUpdated false)
  (Transformation|DetachFromActor "KeepWorld" "KeepWorld" "KeepRelative")
  (CallFunction|DropTrace)
  (Utilities|TogglePhysics true))

(fn ConstructionScript)

(fn DropTrace
  (bind _returnvalue (Transformation|GetActorLocation))
  (bind _returnvalue_2 (Game|GetPlayerCameraManager 0))
  (bind _returnvalue_3 (Camera|GetCameraLocation _returnvalue_2))
  (bind (_outhit _returnvalue_4) (Collision|CapsuleTraceByChannel _returnvalue_3 (+ _returnvalue_3 (* (Math|Vector|GetForwardVector (Camera|GetCameraRotation _returnvalue_2)) 2.5e+02)) 5.0 5.0 "TraceTypeQuery1" true 0 "None"))
  (if _returnvalue_4
    (if (> (Math|Vector|DotProduct (.ImpactNormal (Collision|BreakHitResult _outhit)) "0.000000,0.000000,1.000000") 0.1)
      (Transformation|SetActorLocation (.Location (Collision|BreakHitResult _outhit)) false true)
      (Transformation|SetActorRotation "0, 0, 0")
      (else
        (bind (_outhit_2 _returnvalue_5) (Collision|CapsuleTraceByChannel (.Location (Collision|BreakHitResult _outhit)) (+ (.Location (Collision|BreakHitResult _outhit)) "0.000000,0.000000,-500.000000") 5.0 0.0 "TraceTypeQuery1" true 0 "None"))
        (if _returnvalue_5
          (Transformation|SetActorLocation (.Location (Collision|BreakHitResult _outhit_2)) false true)
          (Transformation|SetActorRotation "0, 0, 0"))))
    (else
      (bind (_outhit_3 _returnvalue_6) (Collision|CapsuleTraceByChannel _returnvalue (+ _returnvalue "0.000000,0.000000,-500.000000") 5.0 5.0 "TraceTypeQuery1" true 0 "None"))
      (if _returnvalue_6
        (Transformation|SetActorLocation (.Location (Collision|BreakHitResult _outhit_3)) false true)
        (Transformation|SetActorRotation "0, 0, 0")))))

(fn GetHandIK
  (return (Transformation|GetWorldLocation (Variables|Default|GetHandIK)) (Transformation|GetWorldLocation (Variables|Default|GetWristIK))))

(fn GetItemSocket
  (return "None"))

(fn IsLeftPickup
  (return false))

(fn IsPickupable
  (return (Variables|Default|GetbCanPickup)))
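; BP_Interactable_Dalla is a left-pickup interactable dallah that refills Finjal cups from a limited Capacity.
; RefillFinjal accepts two Finjal states, subtracts the cup's capacity and calls FillFinjal, then updates the W_DallahCapacity widget.
; If the remainder would be zero or less, it zeroes Capacity without filling; this and invalid states send messages through BP_GameState.
; PickedUp sets the capacity widget's visibility from IsHeld.
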(event Custom|RefillFinjal
  (params (Finjal :type BP%20Interactable%20Cup%20Object%20Reference))
  (bind _finjalstate (Variables|/Game/Game/Blueprints/Gameplay/Items/BP_Interactable_Cup.BP_Interactable_Cup_C|GetFinjalState Finjal))
  (if (or (Utilities|Enum|Equal(Enum) _finjalstate "NewEnumerator3") (Utilities|Enum|Equal(Enum) _finjalstate "NewEnumerator2"))
    (if (<= (- (Variables|Default|GetCapacity) (Variables|/Game/Game/Blueprints/Gameplay/Items/BP_Interactable_Cup.BP_Interactable_Cup_C|GetFinjalCapacity Finjal)) 0.0)
      (bind _asbp_game_state (Utilities|Casting|CastToBP_GameState (Game|GetGameState)))
      (Default|CallOnSendMessage _asbp_game_state "This dallah is empty..." 5.0)
      (Variables|Default|SetCapacity 0.0)
      (else
        (Variables|Default|SetCapacity (- (Variables|Default|GetCapacity) (Variables|/Game/Game/Blueprints/Gameplay/Items/BP_Interactable_Cup.BP_Interactable_Cup_C|GetFinjalCapacity Finjal)))
        (Default|FillFinjal Finjal)))
    (bind _asw_dallah_capacity (Utilities|Casting|CastToW_DallahCapacity (UserInterface|GetWidget (Variables|Default|GetW_Capacity))))
    (Variables|/Game/Game/UI/Gameplay/W_DallahCapacity.W_DallahCapacity_C|SetFinjalCapacity _asw_dallah_capacity (Variables|Default|GetCapacity))
    (else
      (bind _asbp_game_state_2 (Utilities|Casting|CastToBP_GameState (Game|GetGameState)))
      (Default|CallOnSendMessage _asbp_game_state_2 "Can't fill this Finjal currently..." 5.0))))

(event EventBeginPlay
  (|CallParentFunction) ; This node is disabled and will not be called.\nDrag off pins to build functionality.
)

(event Collision|EventActorBeginOverlap
  (params (OtherActor :type Actor%20Object%20Reference))
  (|CallParentFunction OtherActor) ; This node is disabled and will not be called.\nDrag off pins to build functionality.
)

(event EventTick
  (params (DeltaSeconds :type Float%20%28single-precision%29))
  (|CallParentFunction DeltaSeconds) ; This node is disabled and will not be called.\nDrag off pins to build functionality.
)

(event EventPickedUp
  (Rendering|SetVisibility (Variables|Default|GetW_Capacity) (Variables|Default|GetbIsHeld) false))

(fn ConstructionScript
  (|CallParentFunction))

(fn IsLeftPickup
  (return true))
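; Gameplay manager that populates the level with AI customers at startup, then starts the background music.
; On BeginPlay, a custom delayed-loop macro calls SpawnCustomer up to the seated-customer limit, pausing a random short interval between spawns, then fades in the music.
; SpawnCustomer spawns a behavior-tree-driven BP_Customer at AISpawnPoint; its scan of sofa occupancy has no effect.
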(event EventBeginPlay
  (Utilities|ForLoopwithDelayy 1 (Variables|Default|GetMaxSeatedCustomers) (Math|Random|RandomFloatinRange 1.0 2.0) :!label _label
    (:LoopBody
      (CallFunction|SpawnCustomer)
      (goto _label Next))
    (:Completed
      (bind _returnvalue (Audio|SpawnSound2D "/Game/Game/Audio/Music1.Music1" 1.0 1.0 0.0 0))
      (bind _output_get (Variables|Default|SetMusic _returnvalue))
      (Audio|Components|Audio|FadeIn _output_get 5.0 1.0 0.0 "Linear" :!class /Script/Engine.AudioComponent))))

(fn ConstructionScript)

(fn SpawnCustomer
  (bind _aispawnpoint (Variables|Default|GetAISpawnPoint))
  (bind _returnvalue (Transformation|GetActorTransform _aispawnpoint))
  (bind _outactors (Actor|GetAllActorsOfClass "/Game/Game/Blueprints/Gameplay/Level/BP_Sofa.BP_Sofa_C"))
  (for _array_element _outactors
    (if (Variables|/Game/Game/Blueprints/Gameplay/Level/BP_Sofa.BP_Sofa_C|GetbIsOccupied _array_element)
      _))
  (Utilities|Time|ClearTimerbyFunctionName 0 "SpawnCustomer")
  (AI|SpawnAIFromClass "/Game/Game/Blueprints/Character/AI/BP_Customer.BP_Customer_C" "/Game/Game/Blueprints/Character/AI/BT_Customer.BT_Customer" (.location _returnvalue) (.rotation _returnvalue) true 0)
  (return))
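; BP_GameState is the game state that tracks seated customers and enforces a seating limit.
; When a customer sits, it compares the seated list against MaxSeatedCustomers from BP_GameplayManager.
; If full, it clears the passed sofa's occupied flag, broadcasts removal and sends the oldest valid customer out of the room.
; It then broadcasts the newcomer's CustomerData and adds them to the list.
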(event Custom|HandleCustomerSittingDown
  (params (Pawn :type Pawn%20Object%20Reference) (Sofa :type BP%20Sofa%20Object%20Reference))
  (bind _currentseatedcustomers (Variables|Default|GetCurrentSeatedCustomers))
  (bind _output (Utilities|Array|Get(acopy) _currentseatedcustomers))
  ;[1 1 1] Handle customer seated
  (bind _asbp_customer (Utilities|Casting|CastToBP_Customer Pawn))
  (bind _returnvalue (Actor|GetActorOfClass "/Game/Game/Blueprints/Gameplay/BP_GameplayManager.BP_GameplayManager_C"))
  (if (< (Utilities|Array|Length (Variables|Default|GetCurrentSeatedCustomers)) (Variables|/Game/Game/Blueprints/Gameplay/BP_GameplayManager.BP_GameplayManager_C|GetMaxSeatedCustomers _returnvalue))
    _
    (else
      (Utilities|IsValid _output
        (:Is%20Valid
          (Variables|/Game/Game/Blueprints/Gameplay/Level/BP_Sofa.BP_Sofa_C|SetbIsOccupied Sofa false)
          (Default|CallCustomerRemoved _output)
          (Default|ExitRoom _output)
          (Utilities|Array|RemoveIndex (Variables|Default|GetCurrentSeatedCustomers))))))
  (Default|CallCustomerSeated (Variables|/Game/Game/Blueprints/Character/AI/BP_Customer.BP_Customer_C|GetCustomerData _asbp_customer) _asbp_customer)
  (Utilities|Array|Add (Variables|Default|GetCurrentSeatedCustomers) _asbp_customer))

(event EventBeginPlay)

(event EventTick
  (params (DeltaSeconds :type Float%20%28single-precision%29)))

(fn ConstructionScript)